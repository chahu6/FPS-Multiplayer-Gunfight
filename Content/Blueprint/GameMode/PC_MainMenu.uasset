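; Player controller for the main menu that handles the title screen and the switch to the main menu.
; On BeginPlay it creates and shows the GameStart_UI widget and enables the mouse cursor.
; Pressing Space removes that widget, adds MainMenu_UI to the viewport and switches input to UI only.
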(event `self.ReceiveBeginPlay`
  (bind _returnvalue (`|CreateWidget` "/Game/Blueprint/GameUI/GameStart_UI.GameStart_UI_C" self))
  (bind _output_get (set `self.GameStartUI` _returnvalue))
  (`UserWidget.AddToViewport` _output_get 0)
  (set `self.bShowMouseCursor` true))

(event `Key|SpaceBar`
  (params (Key :type "Key Structure"))
  (:`Pressed`
    (`Widget.RemoveFromParent` (`self.GameStartUI`))
    (bind _returnvalue (`|CreateWidget` "/Game/Blueprint/GameUI/MainMenu_UI.MainMenu_UI_C" self))
    (`UserWidget.AddToViewport` _returnvalue 0)
    (`WidgetBlueprintLibrary.SetInputMode_UIOnlyEx` self null)))

(fn `UserConstructionScript`)