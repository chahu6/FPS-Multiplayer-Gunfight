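; Game mode for a timed deathmatch that tracks each player's score, rewarding kills and penalizing deaths.
; The first PostLogin caches PlayerStarts and starts a one-second countdown; every login registers the controller in a score map and starts its spawn flow.
; Spawn requests create BP_Attack characters at start points in round-robin order.
; Score changes, timer ticks and round end are pushed to every mapped controller.
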(event `KillAnother`
  (params (PlayerController :type "/Game/Blueprint/GameMode/BP_FPSPlayerController Object Reference"))
  (bind _playergamedatamap (`self.PlayerGameDataMap`))
  (bind (_value _returnvalue) (`BlueprintMapLibrary.Map_Find` (`self.PlayerGameDataMap`) PlayerController))
  (if _returnvalue
    (bind _output_get (set `self.NewVar_1` _value))
    (bind (_playername _playerscore) (break `DeathMatchPlayerData` _output_get))
    (set `self.NewVar_1` (make `DeathMatchPlayerData` _playername (+ _playerscore 15)))
    (`BlueprintMapLibrary.Map_Remove` _playergamedatamap PlayerController)
    (`BlueprintMapLibrary.Map_Add` _playergamedatamap PlayerController (`self.NewVar_1`))
    (`self.UpdateValues`)
    (else
      (`KismetSystemLibrary.PrintString` "失败" :!label _label))))

(event `SelfDeath`
  (params (PlayerController :type "/Game/Blueprint/GameMode/BP_FPSPlayerController Object Reference"))
  (bind _playergamedatamap (`self.PlayerGameDataMap`))
  (bind (_value _returnvalue) (`BlueprintMapLibrary.Map_Find` (`self.PlayerGameDataMap`) PlayerController))
  (if _returnvalue
    (bind _output_get (set `self.NewVar_0` _value))
    (bind (_playername _playerscore) (break `DeathMatchPlayerData` _output_get))
    (set `self.NewVar_0` (make `DeathMatchPlayerData` _playername (- _playerscore 10)))
    (`BlueprintMapLibrary.Map_Remove` _playergamedatamap PlayerController)
    (`BlueprintMapLibrary.Map_Add` _playergamedatamap PlayerController (`self.NewVar_0`))
    (`self.UpdateValues`)
    (else
      (goto _label))))

(event `self.K2_PostLogin`
  (params (NewPlayer :type "PlayerController Object Reference"))
  (if (not (`self.IsFirstJoin`))
    (`self.GameStateSet`)
    (set `self.IsFirstJoin` true))
  (bind _asbp_fpsplayer_controller (cast `/Game/Blueprint/GameMode/BP_FPSPlayerController` NewPlayer))
  (`/Game/Blueprint/GameMode/BP_FPSPlayerController.StartSpawnCharacter` _asbp_fpsplayer_controller)
  (`BlueprintMapLibrary.Map_Add` (`self.PlayerGameDataMap`) _asbp_fpsplayer_controller (make `DeathMatchPlayerData` (`KismetStringLibrary.Conv_StringToName` (`KismetSystemLibrary.GetObjectName` _asbp_fpsplayer_controller)))))

(event `GameStateSet`
  (bind _outactors (`GameplayStatics.GetAllActorsOfClass` "/Script/Engine.PlayerStart"))
  (set `self.CharacterSpawnPoints` _outactors)
  (bind _returnvalue (`KismetSystemLibrary.K2_SetTimerDelegate` (delegate `Down`) 1.0 true))
  (set `self.TimerHandle` _returnvalue))

(event `Down`
  (bind _result (`/Engine/EditorBlueprintResources/StandardMacros.DecrementInt` (`self.RoundTime`))
    (:`  `
      (bind _keys (`BlueprintMapLibrary.Map_Keys` (`self.PlayerGameDataMap`)))
      (for _array_element _keys
        (`/Game/Blueprint/GameMode/BP_FPSPlayerController.ClientUpdateTime` _array_element _result))
      (if (<= (`self.RoundTime`) 0)
        (`KismetSystemLibrary.K2_ClearAndInvalidateTimerHandle` (`self.TimerHandle`))
        (`self.EndGame`)))))

(event `RequestSpawn`
  (params (PlayerController :type "/Game/Blueprint/GameMode/BP_FPSPlayerController Object Reference"))
  (`/Game/Blueprint/GameMode/BP_FPSPlayerController.SpawnPlayerCharacter` PlayerController "/Game/Blueprint/Player/BP_Attack.BP_Attack_C" (`self.GetTransform` (`|GetArrayItem` (`self.CharacterSpawnPoints`) (`self.SpawnIndex`))))
  (bind _result (`/Engine/EditorBlueprintResources/StandardMacros.IncrementInt` (`self.SpawnIndex`))
    (:`  `
      (set `self.SpawnIndex` _result)
      (if (>= (`self.SpawnIndex`) (`KismetArrayLibrary.Array_Length` (`self.CharacterSpawnPoints`)))
        (set `self.SpawnIndex` 0)))))

(event `UpdateValues`
  (bind _playergamedatamap (`self.PlayerGameDataMap`))
  (bind _keys (`BlueprintMapLibrary.Map_Keys` _playergamedatamap))
  (for _array_element _keys
    (bind _values (`BlueprintMapLibrary.Map_Values` _playergamedatamap))
    (`/Game/Blueprint/GameMode/BP_FPSPlayerController.UpdateValues` _array_element _values)))

(event `EndGame`
  (bind _keys (`BlueprintMapLibrary.Map_Keys` (`self.PlayerGameDataMap`)))
  (for _array_element _keys
    (`/Game/Blueprint/GameMode/BP_FPSPlayerController.ClientEndGame` _array_element)))

(fn `UserConstructionScript`)