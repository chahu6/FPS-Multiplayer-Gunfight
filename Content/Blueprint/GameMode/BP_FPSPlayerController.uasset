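; Player controller for an FPS deathmatch, linking the DeathMatchGameMode to the local player's HUD.
; On death it reports the death and the killer's controller to the game mode, then requests a respawn after a delay; spawning possesses a new pawn and switches to game-only input.
; It creates the Player_UI widget locally and forwards scoreboard, ammo, health and crosshair recoil updates to it.
; It also stores the countdown time and returns to MainMenu at game end.
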(event `ClientEndGame`
  (`GameplayStatics.OpenLevel` "MainMenu"))

(event `ClientUpdateTime`
  (params (CountDownTime :type Integer))
  (set `self.CountDownTime` CountDownTime))

(event `self.DeathMatch`
  (params (DamageActor :type "Actor Object Reference"))
  (bind _asdeath_match_game_mode (cast `/Game/Blueprint/GameMode/DeathMatchGameMode` (`GameplayStatics.GetGameMode`)))
  (`/Game/Blueprint/GameMode/DeathMatchGameMode.SelfDeath` _asdeath_match_game_mode self)
  (bind _asbp_fpsplayer_controller (cast `/Game/Blueprint/GameMode/BP_FPSPlayerController` (`self.GetInstigatorController` DamageActor)))
  (`/Game/Blueprint/GameMode/DeathMatchGameMode.KillAnother` _asdeath_match_game_mode _asbp_fpsplayer_controller)
  (`KismetSystemLibrary.Delay` 3.0)
  (bind _asdeath_match_game_mode_2 (cast `/Game/Blueprint/GameMode/DeathMatchGameMode` (`GameplayStatics.GetGameMode`)))
  (`/Game/Blueprint/GameMode/DeathMatchGameMode.RequestSpawn` _asdeath_match_game_mode_2 self))

(event `ServerRequireUpdateValues`
  (bind _asdeath_match_game_mode (cast `/Game/Blueprint/GameMode/DeathMatchGameMode` (`GameplayStatics.GetGameMode`)))
  (`/Game/Blueprint/GameMode/DeathMatchGameMode.UpdateValues` _asdeath_match_game_mode))

(event `UpdateValues`
  (params (Values :type "Array of DeathMatchPlayerData Structure"))
  (bind _output_get (set `self.Values` Values))
  (`KismetMultiFPSLibrary.SortValues` _output_get)
  (bind _playerui (`self.PlayerUI`)
    (:`then`
      (`/Game/Blueprint/GameUI/Player_UI.UpdateSortBox` _playerui (`self.Values`)))
    (:`else`)))

(event `ClientHideMouse`
  (`WidgetBlueprintLibrary.SetInputMode_GameOnly` self)
  (set `self.bShowMouseCursor` false))

(event `SpawnPlayerCharacter`
  (params (Class :type "/Game/Blueprint/Player/BP_Attack Class Reference") (SpawnTransform :type "Transform Structure"))
  (bind _returnvalue (`|SpawnActorFromClass` Class SpawnTransform "Undefined" "OverrideRootScale" null null))
  (`self.Possess` _returnvalue)
  (`self.ClientHideMouse`))

(event `StartSpawnCharacter`
  (`KismetSystemLibrary.Delay` 1.0)
  (bind _asdeath_match_game_mode (cast `/Game/Blueprint/GameMode/DeathMatchGameMode` (`GameplayStatics.GetGameMode`)))
  (`/Game/Blueprint/GameMode/DeathMatchGameMode.RequestSpawn` _asdeath_match_game_mode self))

(event `self.CreatePlayerUI`
  ;[1 1 1] UI
  (`self.PlayerUI`
    (:`then`
      (`Widget.RemoveFromParent` (`self.PlayerUI`)))
    (:`else`
      _))
  (if (`self.IsLocalController`)
    (bind _returnvalue (`|CreateWidget` "/Game/Blueprint/GameUI/Player_UI.Player_UI_C" self))
    (bind _output_get (set `self.PlayerUI` _returnvalue))
    (`UserWidget.AddToViewport` _output_get 0)
    (`self.ServerRequireUpdateValues`)))

(event `self.DoCrosshairRecoil`
  (bind _playerui (`self.PlayerUI`))
  ;[1 1 1] UI
  (`/Engine/EditorBlueprintResources/StandardMacros.IsValid` _playerui
    (:`Is Valid`
      (`/Game/Blueprint/GameUI/Player_UI.DoCrosshair` _playerui))
    (:`Is Not Valid`
      (`KismetSystemLibrary.PrintString` "一样"))))

(event `self.UpdateAmmoUI`
  (params (ClipCurrentAmmo :type Integer) (GunCurrentAmmo :type Integer))
  (bind _playerui (`self.PlayerUI`))
  ;[1 1 1] UI
  (`/Engine/EditorBlueprintResources/StandardMacros.IsValid` _playerui
    (:`Is Valid`
      (`/Game/Blueprint/GameUI/Player_UI.UpdateAmmo` _playerui ClipCurrentAmmo GunCurrentAmmo))
    (:`Is Not Valid`
      (`KismetSystemLibrary.PrintString` "UI改不了"))))

(event `self.UpdateHealthUI`
  (params (NewHealth :type "Float (single-precision)"))
  (bind _playerui (`self.PlayerUI`))
  ;[1 1 1] UI
  (`/Engine/EditorBlueprintResources/StandardMacros.IsValid` _playerui
    (:`Is Valid`
      (`/Game/Blueprint/GameUI/Player_UI.UpdateHealth` _playerui NewHealth))
    (:`Is Not Valid`
      (`KismetSystemLibrary.PrintString` "哇哦操"))))

(fn `UserConstructionScript`)